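; First-person player character for what appears to be a horror game, able to switch between its own view and the level's surveillance cameras.
; Camera mode gathers every BP_camera, drives a HUD with static noise, and turns MoveRight into camera panning.
; Line traces handle key pickup and exit doors, pausing to show messages.
; Enemy damage forces cameras closed, can hand the view to a holding enemy, and leads to timed recovery or death.
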(event Custom|E_switchCamera
  (params (cameraActorRef :type Camera%20Actor%20Object%20Reference))
  (Utilities|MCameraNoise)
  (01.camera|FSwichCamera cameraActorRef))

(event EventBeginPlay
  (Utilities|MGetAllCamera)
  (Utilities|MCreateHud))

(event Collision|EventActorBeginOverlap
  (params (OtherActor :type Actor%20Object%20Reference)))

(event EventTick
  (params (DeltaSeconds :type Float%20%28single-precision%29))
  (if (Variables|Default|GetisHold)
    (Utilities|IsValid (Variables|Default|GetenemyRef)
      (:Is%20Valid
        (Utilities|FlowControl|Sequence
          (:then_0
            (Utilities|FlowControl|DoOnce false :!label _label
              (:Completed
                (Input|EnableInput (Game|GetPlayerController 0))
                (bind _asbp_hearing_enemy (Utilities|Casting|CastToBP_HearingEnemy (Variables|Default|GetenemyRef)))
                (Utilities|FlowControl|Delay 0.5)
                (Game|Player|SetViewTargetwithBlend (Game|GetPlayerController 0) _asbp_hearing_enemy 0.0 "VTBlend_Linear" 0.0 false))))
          (:then_1
            (bind _ishold (Class|BPIEnemy|FIGetIsHolding(Message) (Variables|Default|GetenemyRef)))
            (bind _output_get (Variables|Default|SetisHold _ishold))
            (if (not _output_get)
              (Game|Player|SetViewTargetwithBlend (Game|GetPlayerController 0) (Game|GetPlayerCharacter 0) 0.0 "VTBlend_Linear" 0.0 false))))))
    (else
      (goto _label Reset))))

(event Input|ActionEvents|InputActionSprint
  (params (Key :type Key%20Structure :default "None"))
  (bind _charactermovement (Variables|Character|GetCharacterMovement))
  ;[1 1 1] 走る
  (:Pressed
    (Variables|/Script/Engine.CharacterMovementComponent|SetMaxWalkSpeed _charactermovement (Variables|02.movement|GetsprintSpeed)))
  (:Released
    (Variables|/Script/Engine.CharacterMovementComponent|SetMaxWalkSpeed _charactermovement (Variables|02.movement|GetwalkSpeed))))

(event Input|ActionEvents|InputActionswitichView
  (params (Key :type Key%20Structure :default "None"))
  ;[1 1 1] 視点切り替え
  (:Pressed
    (if (Variables|01.camera|GetisPlayerCamera)
      (Utilities|MCameraOpen)
      (else
        (Utilities|MCameraClose)))))

(event Input|ActionEvents|InputActionAction
  (params (Key :type Key%20Structure :default "None"))
  (bind _playercamera (Variables|Default|GetplayerCamera))
  (bind _returnvalue (Transformation|GetWorldLocation _playercamera))
  ;[1 1 1] アクションボタン
  (:Pressed
    (if (Variables|01.camera|GetisPlayerCamera)
      (bind (_outhit _returnvalue_2) (Collision|LineTraceByChannel _returnvalue (+ _returnvalue (* (Math|Vector|GetForwardVector _playercamera) 1e+03)) "TraceTypeQuery1" false 0 "None"))
      (if _returnvalue_2
        (if (Game|IsGamePaused)
          (Game|SetGamePaused false)
          (Default|EOutputText (Variables|03.widget|GetplayerHudWidgetRef))
          (else
            (bind _ishitobject (03.object|FObjectAction (.HitActor (Collision|BreakHitResult _outhit))))
            (if _ishitobject
              (Game|SetGamePaused true))))))))

(event Input|AxisEvents|InputAxisMoveForward
  (params (AxisValue :type Float%20%28single-precision%29))
  ;[1 1 1] 移動
  (if (Variables|01.camera|GetisPlayerCamera)
    (Pawn|Input|AddMovementInput (Math|Vector|GetForwardVector (Math|Rotator|MakeRotator 0.0 0.0 (.yaw (Pawn|GetControlRotation (Class|PawnMovementComponent|GetPawnOwner (Variables|Character|GetCharacterMovement)) :!class /Script/Engine.Pawn)))) AxisValue false)
    (02.movement|FHeadShake)
    (02.movement|FFootStep)))

(event Input|AxisEvents|InputAxisMoveRight
  (params (AxisValue :type Float%20%28single-precision%29))
  (bind _cameraactors (Variables|01.camera|GetcameraActors))
  (bind _currentcameranum (Variables|01.camera|GetcurrentCameraNum))
  (bind _output (Utilities|Array|Get(acopy) _cameraactors _currentcameranum))
  ;[1 1 1] 移動
  (if (Variables|01.camera|GetisPlayerCamera)
    (Pawn|Input|AddMovementInput (Math|Vector|GetRightVector (Math|Rotator|MakeRotator 0.0 0.0 (.yaw (Pawn|GetControlRotation (Class|PawnMovementComponent|GetPawnOwner (Variables|Character|GetCharacterMovement)) :!class /Script/Engine.Pawn)))) AxisValue false)
    (02.movement|FHeadShake)
    (02.movement|FFootStep)
    (else
      (Utilities|IsValid _output
        (:Is%20Valid
          (Default|EShakeHead _output (Input|AxisValues|GetMoveRight)))))))

(event Input|AxisEvents|InputAxisLookUp
  (params (AxisValue :type Float%20%28single-precision%29))
  ;[1 1 1] カメラ操作（マウス）
  (if (Variables|01.camera|GetisPlayerCamera)
    (Pawn|Input|AddControllerPitchInput (* AxisValue (Variables|01.camera|GetcameraSensitivity)))))

(event Input|AxisEvents|InputAxisTurn
  (params (AxisValue :type Float%20%28single-precision%29))
  ;[1 1 1] カメラ操作（マウス）
  (if (Variables|01.camera|GetisPlayerCamera)
    (Pawn|Input|AddControllerYawInput (* AxisValue (Variables|01.camera|GetcameraSensitivity)))))

(event Game|Damage|EventAnyDamage
  (params (Damage :type Float%20%28single-precision%29) (DamageType :type Damage%20Type%20Object%20Reference) (InstigatedBy :type Controller%20Object%20Reference) (DamageCauser :type Actor%20Object%20Reference))
  (bind _playerhudwidgetref (Variables|03.widget|GetplayerHudWidgetRef))
  (Utilities|FlowControl|Delay 0.2)
  (bind _asbp_enemy (Utilities|Casting|CastToBP_enemy DamageCauser))
  (Variables|Default|SetenemyRef _asbp_enemy)
  (if (> (Variables|05.status|GethitPoint) 0.0)
    (bind _ishold (Class|BPIEnemy|FIGetIsHolding(Message) (Variables|Default|GetenemyRef)))
    (Variables|Default|SetisHold _ishold)
    (Variables|05.status|SethitPoint (- (Variables|05.status|GethitPoint) Damage))
    (if (Variables|01.camera|GetisPlayerCamera)
      _
      (else
        (01.camera|FForcedClose)))
    (if (<= (Variables|05.status|GethitPoint) 0.0)
      (Variables|05.status|SetisDead true)
      (Default|EIsDamage (Variables|03.widget|GetplayerHudWidgetRef) true)
      (Audio|PlaySound2D "/Game/workspace/1_mainGame/a_sound/Death_Cue.Death_Cue" 1.0 1.0 0.0 0 0)
      (Input|EnableInput (Game|GetPlayerController 0))
      (Transformation|AttachComponentToComponent (Variables|Default|GetplayerCamera) (Variables|Default|GetdeadCameraPos) "None" "SnapToTarget" "SnapToTarget" "SnapToTarget" true)
      (Collision|SetCollisionEnabled (Variables|Collision|GetCapsuleComponent) "NoCollision")
      (Utilities|FlowControl|Delay 3.0)
      (UserInterface|Animation|PlayAnimation _playerhudwidgetref (Variables|/Game/workspace/1_mainGame/9_widget/WBP_playerHud.WBP_playerHud_C|GetdeadFade _playerhudwidgetref) 0.0 1 "Forward" 1.0 false)
      (Utilities|FlowControl|Delay 3.0)
      (Default|FSetDead (Variables|03.widget|GetplayerHudWidgetRef) true)
      (Utilities|IsValid (Variables|Default|GetcameraNoise)
        (:Is%20Not%20Valid
          (bind _returnvalue (Audio|CreateSound2D "/Game/workspace/1_mainGame/a_sound/TvNoise.TvNoise" 0.5 1.0 0.0 0))
          (bind _output_get (Variables|Default|SetcameraNoise _returnvalue))
          (Audio|Components|Audio|Play _output_get 0.0)))
      (else
        (04.damage|FDamage)
        (Utilities|FlowControl|RetriggerableDelay 1e+01)
        (04.damage|FRecovery)))))

(fn ConstructionScript
  (Components|SkinnedMesh|HideBonebyName (Variables|Character|GetMesh) "head" "PBO_None"))

(fn FHeadShake
  (if (>= (02.movement|FGetMovementLength) (LocalVariables|Getis_shake_length))
    (Class|PlayerController|ClientPlayCameraShake (Game|GetPlayerController 0) "/Game/workspace/1_mainGame/1_player/BP_shakeWalking.BP_shakeWalking_C" (Utilities|MShakeScale) "CameraLocal" "0, 0, 0")))

(fn FGetMovementLength
  (return (Math|Vector|VectorLength (Variables|/Script/Engine.MovementComponent|GetVelocity (Pawn|GetMovementComponent (Game|Player|GetPlayerPawn 0))))))

(fn FChangeCamera
  (Game|Player|SetViewTargetwithBlend (Game|GetPlayerController 0) (select (Variables|01.camera|GetisPlayerCamera) (Game|GetPlayerCharacter 0) (Utilities|Array|Get(acopy) (Variables|01.camera|GetcameraActors) (Variables|01.camera|GetcurrentCameraNum))) 0.0 "VTBlend_Linear" 0.0 false)
  (for (_array_element _array_index) (Variables|01.camera|GetcameraActors)
    (Default|FSetActive _array_element (== _array_index (Variables|01.camera|GetcurrentCameraNum)))))

(fn FSwichCamera
  (params (cameraActorRef :type Camera%20Actor%20Object%20Reference))
  (bind _asbp_camera (Utilities|Casting|CastToBP_camera cameraActorRef))
  (Variables|01.camera|SetcameraRef _asbp_camera)
  (Variables|01.camera|SetcurrentCameraNum (Utilities|Array|FindItem (Variables|01.camera|GetcameraActors) (Variables|01.camera|GetcameraRef)))
  (Utilities|FlowControl|Sequence
    (:then_0
      (for (_array_element _array_index) (Variables|01.camera|GetcameraActors)
        (Default|FSetActive _array_element (== _array_index (Variables|01.camera|GetcurrentCameraNum)))))
    (:then_1
      (Game|Player|SetViewTargetwithBlend (Game|GetPlayerController 0) _asbp_camera 0.0 "VTBlend_Linear" 0.0 false)
      (Default|FGetCameraType (Variables|03.widget|GethudWidgetRef) (Variables|/Game/workspace/1_mainGame/4_camera/BP_camera.BP_camera_C|GetcameraType (Variables|01.camera|GetcameraRef)))
      (Default|FChangeCameraColor (Variables|03.widget|GethudWidgetRef) (Variables|01.camera|GetcurrentCameraNum))
      (01.camera|FSpawnSoundCameraNoise))))

(fn FFootStep
  (bind _returnvalue (Game|GetPlayerCharacter 0))
  (bind _returnvalue_2 (Transformation|GetActorLocation _returnvalue))
  (if (and (> (Math|Vector|VectorLength (- (Transformation|GetActorLocation (Game|GetPlayerCharacter 0)) (Variables|02.movement|GetcurrentFootLocation))) (LocalVariables|GetstepSize)) (>= (Math|Vector|VectorLength (Variables|/Script/Engine.MovementComponent|GetVelocity (Pawn|GetMovementComponent (Game|Player|GetPlayerPawn 0)))) 5e+01))
    (bind (_outhit _returnvalue_3) (Collision|SphereTraceByChannel _returnvalue_2 (- _returnvalue_2 "0, 0,150.000000") 0.0 "TraceTypeQuery1" false 0 "None"))
    (if _returnvalue_3
      (Audio|SpawnSoundatLocation "/Game/workspace/1_mainGame/a_sound/Rock_Cue.Rock_Cue" (.Location (Collision|BreakHitResult _outhit)) "0, 0, 0" (Variables|04.sound|GetfootStepSoundVolume) 1.0 0.0 "/Game/workspace/1_mainGame/a_sound/SA_enviroment.SA_enviroment" 0)
      (Variables|02.movement|SetcurrentFootLocation (.Location (Collision|BreakHitResult _outhit))))))

(fn FExitDoorOpen
  (params (hitActorRef :type Actor%20Object%20Reference))
  (Class|BPIObjectInfo|FIExitDoorOpen(Message) hitActorRef))

(fn FExitDoorClose
  (params (hitActorRef :type Actor%20Object%20Reference))
  (Class|BPIObjectInfo|FIExitDoorClose(Message) hitActorRef)
  (Default|EOutputText (Variables|03.widget|GetplayerHudWidgetRef) "鍵がかかっている"))

(fn FCameraShakeHead
  (bind _cameraactors (Variables|01.camera|GetcameraActors))
  (bind _currentcameranum (Variables|01.camera|GetcurrentCameraNum))
  (bind _output (Utilities|Array|Get(acopy) _cameraactors _currentcameranum))
  (Utilities|IsValid _output
    (:Is%20Valid
      (Default|EShakeHead _output (Input|AxisValues|GetMoveRight)))))

(fn FGetKey
  (Variables|07.object|SethasKey true)
  (Actor|DestroyActor (Variables|07.object|GethitActorRef))
  (Default|EOutputText (Variables|03.widget|GetplayerHudWidgetRef) "鍵を入手した"))

(fn FObjectAction
  (params (hitActorRef :type Actor%20Object%20Reference))
  (Variables|07.object|SethitActorRef hitActorRef)
  (Utilities|MCasttoObject (Variables|07.object|GethitActorRef)
    (:key
      (03.object|FGetKey)
      (return true))
    (:exitDoor
      (if (Variables|07.object|GethasKey)
        (03.object|FExitDoorOpen (Variables|07.object|GethitActorRef))
        (else
          (03.object|FExitDoorClose (Variables|07.object|GethitActorRef))
          (return true))))
    (:null
      (return false))))

(fn FSpawnSoundCameraNoise
  (Utilities|IsValid (Variables|01.camera|GetcameraRef)
    (:Is%20Valid
      (if (Utilities|Enum|Equal(Enum) (Variables|/Game/workspace/1_mainGame/4_camera/BP_camera.BP_camera_C|GetcameraType (Variables|01.camera|GetcameraRef)) "NewEnumerator1")
        (bind _returnvalue (Audio|CreateSound2D "/Game/workspace/1_mainGame/a_sound/TvNoise.TvNoise" 0.1 0.7 0.0 0))
        (bind _output_get (Variables|Default|SetcameraNoise _returnvalue))
        (Audio|Components|Audio|Play _output_get 0.0)
        (else
          (Utilities|IsValid (Variables|Default|GetcameraNoise)
            (:Is%20Valid
              (if (Audio|Components|Audio|IsPlaying (Variables|Default|GetcameraNoise))
                (Audio|Components|Audio|Stop (Variables|Default|GetcameraNoise))))))))))

(fn FDamage
  (Default|EIsDamage (Variables|03.widget|GetplayerHudWidgetRef) true)
  (Class|PlayerController|ClientPlayCameraShake (Game|GetPlayerController 0) "/Game/workspace/1_mainGame/1_player/BP_shakeDamage.BP_shakeDamage_C" 1.0 "CameraLocal" "0, 0, 0")
  (Audio|PlaySound2D "/Game/workspace/1_mainGame/a_sound/Damage_Cue.Damage_Cue" 1.0 1.0 0.0 0 0)
  (Audio|PlaySound2D "/Game/workspace/1_mainGame/a_sound/Heartbeat_Cue.Heartbeat_Cue" 0.5 1.0 0.0 0 0))

(fn FRecovery
  (Variables|05.status|SethitPoint 0.3)
  (Default|EIsDamage (Variables|03.widget|GetplayerHudWidgetRef) false))

(fn FForcedClose
  (Variables|01.camera|SetisPlayerCamera true)
  (Widget|SetVisibility (Variables|03.widget|GethudWidgetRef) "Hidden")
  (Input|SetInputModeGameOnly (Game|GetPlayerController 0))
  (Variables|/Script/Engine.PlayerController|SetbShowMouseCursor (Game|GetPlayerController 0) false)
  (Components|SkinnedMesh|HideBonebyName (Variables|Character|GetMesh) "head" "PBO_None")
  (01.camera|FChangeCamera)
  (Default|FChangeCameraColor (Variables|03.widget|GethudWidgetRef) (Variables|01.camera|GetcurrentCameraNum))
  (Default|FSetActive (Utilities|Array|Get(acopy) (Variables|01.camera|GetcameraActors) (Variables|01.camera|GetcurrentCameraNum)) false))

(fn FIGetViewCamera
  (return (Utilities|Array|Get(acopy) (Variables|01.camera|GetcameraActors) (Variables|01.camera|GetcurrentCameraNum))))

(fn FIIsDead
  (return (Variables|05.status|GetisDead)))

(fn FIIsViewCamera
  (return (not (Variables|01.camera|GetisPlayerCamera))))