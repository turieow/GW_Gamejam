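; BP_EventDoor is a door actor with a Paper2D sprite that swings shut when its E_Close event is called.
; E_Close plays a creaking sound with environment attenuation at the sprite's X and Z and the actor's Y, then runs the TL_Close timeline.
; The timeline's Close track sets the actor's yaw each update, keeping pitch and roll unchanged.
; The Blueprint contains no opening logic or trigger of its own.
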(event Custom|E_Close
  (bind _returnvalue (Transformation|GetActorRotation))
  (bind _papersprite (Variables|Default|GetPaperSprite))
  (bind _returnvalue_2 (Transformation|GetWorldLocation _papersprite))
  (Audio|PlaySoundatLocation "/Game/workspace/1_mainGame/a_sound/Creaking_door_2.Creaking_door_2" (Math|Vector|MakeVector (.x _returnvalue_2) (.y (Transformation|GetActorLocation)) (.z _returnvalue_2)) "0, 0, 0" 1.0 1.0 0.0 "/Game/workspace/1_mainGame/a_sound/SA_enviroment.SA_enviroment" 0 0)
  (bind _close (Timeline|TL_Close Play)
    (:Update
      (Transformation|SetActorRotation (Math|Rotator|MakeRotator (.roll _returnvalue) (.pitch _returnvalue) _close)))))

(event EventBeginPlay
  (|CallParentFunction) ; このノードは無効になっているため呼び出せません。\n機能をビルドするにはピンをドラッグしてください。
)

(event Collision|EventActorBeginOverlap
  (params (OtherActor :type Actor%20Object%20Reference)))

(fn ConstructionScript
  (|CallParentFunction))