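; BP_exitDoor is an exit door actor that swings open when its FIExitDoorOpen event is called.
; The event plays the DoorOpen timeline, whose RotationZ track drives the yaw of the whole actor's relative rotation, with roll and pitch held at zero.
; When the timeline finishes, the Collision component's collision is disabled.
; BeginPlay, overlap and Tick are unused stubs.
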(event EventBeginPlay
  (|CallParentFunction) ; このノードは無効になっているため呼び出せません。\n機能をビルドするにはピンをドラッグしてください。
)

(event Collision|EventActorBeginOverlap
  (params (OtherActor :type Actor%20Object%20Reference))
  (|CallParentFunction OtherActor) ; このノードは無効になっているため呼び出せません。\n機能をビルドするにはピンをドラッグしてください。
)

(event EventTick
  (params (DeltaSeconds :type Float%20%28single-precision%29))
  (|CallParentFunction DeltaSeconds) ; このノードは無効になっているため呼び出せません。\n機能をビルドするにはピンをドラッグしてください。
)

(event EventFIExitDoorOpen
  (bind _rotation_z (Timeline|DoorOpen Play)
    (:Update
      (Transformation|SetActorRelativeRotation (Math|Rotator|MakeRotator 0.0 0.0 _rotation_z)))
    (:Finished
      (Collision|SetCollisionEnabled (Variables|Default|Getcollision) "NoCollision"))))

(fn ConstructionScript
  (|CallParentFunction))