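; BP_camera is a camera Blueprint that pans its camera's yaw left and right, like a head shake, within a limited range.
; BeginPlay derives symmetric limits from the local range.
; E_shakeHead checks the accumulated offset against the limit for the input's sign, then rotates via the M_moveYaw macro and advances the offset with constant-speed interpolation.
; F_maxShakeHead builds a limit-based rotation but is never called here.
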(event Custom|E_shakeHead
  (params (axisValue :type Float%20%28single-precision%29))
  (bind _output_get (Variables|Default|SetaxisValue axisValue))
  (if (> _output_get 0.0)
    (if (CallFunction|FIsOverShakeHead 1.0)
      (Transformation|SetWorldRotation (Variables|CameraActor|GetCameraComponent) (Utilities|MMoveYaw (Variables|Default|GetaxisValue)) false false)
      (Variables|Default|SetshakeHeadValue (Math|Interpolation|FInterptoConstant (Variables|Default|GetshakeHeadValue) (+ (Variables|Default|GetshakeHeadValue) (Variables|Default|GetaxisValue)) (Utilities|Time|GetWorldDeltaSeconds) (Variables|Default|GetshakeHeadSpeed)) :!label _label))
    (elif (CallFunction|FIsOverShakeHead -1.0)
      (Transformation|SetWorldRotation (Variables|CameraActor|GetCameraComponent) (Utilities|MMoveYaw (Variables|Default|GetaxisValue)) false false)
      (goto _label))))

(event EventBeginPlay
  (bind _shakeheadlocalrange (Variables|Default|GetshakeHeadlocalRange))
  (Variables|Default|SetshakeHeadWorldRangeRight _shakeheadlocalrange)
  (Variables|Default|SetshakeHeadWorldRangeLeft (* _shakeheadlocalrange -1.0)))

(event Collision|EventActorBeginOverlap
  (params (OtherActor :type Actor%20Object%20Reference)))

(event EventTick
  (params (DeltaSeconds :type Float%20%28single-precision%29)))

(fn ConstructionScript)

(fn FIsOverShakeHead
  (params (isRight :type Float%20%28single-precision%29))
  (if (> isRight 0.0)
    (return (< (Variables|Default|GetshakeHeadValue) (Variables|Default|GetshakeHeadWorldRangeRight)))
    (else
      (return (> (Variables|Default|GetshakeHeadValue) (Variables|Default|GetshakeHeadWorldRangeLeft))))))

(fn FMaxShakeHead
  (params (isRight :type Float%20%28single-precision%29))
  (bind _cameracomponent (Variables|CameraActor|GetCameraComponent))
  (bind _returnvalue (Transformation|GetWorldRotation _cameracomponent))
  (return (Math|Rotator|MakeRotator (.roll _returnvalue) (.pitch _returnvalue) (- (Variables|Default|GetshakeHeadWorldRangeRight) isRight))))