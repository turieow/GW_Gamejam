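; Base object Blueprint with a pulsing emissive mesh and an optional floating icon sprite.
; When HasIcon is set, a looping timer alternates the Paper2D icon between two sprites, and Tick turns it toward the player with pitch locked.
; Tick also ramps the material's Emissive scalar up and down, using the IsEmissive flag to reverse direction at each threshold.
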(event Custom|E_ChangeSprite
  (bind _sprite (Variables|Default|Getsprite))
  (bind _papersprite (Variables|Default|GetPaperSprite))
  (Utilities|FlowControl|FlipFlop
    (:A
      (Rendering|Components|Sprite|SetSprite _papersprite (Utilities|Array|Get(acopy) _sprite)))
    (:B
      (Rendering|Components|Sprite|SetSprite _papersprite (Utilities|Array|Get(acopy) _sprite 1)))))

(event EventBeginPlay
  (if (Variables|Default|GetHasIcon)
    (Utilities|Time|SetTimerbyEvent (delegate Custom|E_ChangeSprite) 0.5 true)))

(event EventTick
  (params (DeltaSeconds :type Float%20%28single-precision%29))
  (CallFunction|FFaceIcon)
  (bind _output_get (Variables|Default|SetemissiveValue (CallFunction|FEmissiveValue)))
  (Rendering|Material|SetScalarParameterValueonMaterials (Variables|Default|Getobject) "Emissive" _output_get)
  (if (and (>= (Variables|Default|GetemissiveValue) 1.0) (not (Variables|Default|GetisEmissive)))
    (Variables|Default|SetisEmissive true)
    (elif (and (<= (Variables|Default|GetemissiveValue) -0.5) (Variables|Default|GetisEmissive))
      (Variables|Default|SetisEmissive false))))

(fn ConstructionScript)

(fn FEmissiveValue
  (return (Math|Interpolation|FInterptoConstant (Variables|Default|GetemissiveValue) (select (Variables|Default|GetisEmissive) (- (Variables|Default|GetemissiveValue) (Utilities|Time|GetWorldDeltaSeconds)) (+ (Variables|Default|GetemissiveValue) (Utilities|Time|GetWorldDeltaSeconds))) (Utilities|Time|GetWorldDeltaSeconds) 5.0)))

(fn FFaceIcon
  (bind _returnvalue (Game|Player|GetPlayerPawn 0))
  (bind _papersprite (Variables|Default|GetPaperSprite))
  (bind _returnvalue_2 (Transformation|GetWorldLocation _papersprite))
  (bind _returnvalue_3 (Transformation|GetActorLocation _returnvalue))
  (bind _returnvalue_4 (Math|Rotator|FindLookatRotation _returnvalue_2 _returnvalue_3))
  (if (Variables|Default|GetHasIcon)
    (Transformation|SetWorldRotation (Variables|Default|GetPaperSprite) (Math|Rotator|MakeRotator (.roll _returnvalue_4) 0.0 (- (.yaw _returnvalue_4) 9e+01)) false false)))