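; Main game mode that counts collected keys and tracks whether a sequence is playing.
; On BeginPlay it sets the view target to the player character, caches all BP_Light actors and binds to its OnGetKey dispatcher.
; Interface calls increment the key count and broadcast it; the first key sends every light a disable message.
; The sequence-playing flag is set and read through interface functions, with a leftover debug print on set.
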(event Custom|E_OnGetKey
  (params (keyNum :type Integer))
  (switch int keyNum
    (:1
      (for _array_element (Variables|Default|GetLights)
        (Class|BPIObjectInfo|FILightEnable(Message) _array_element false)))))

(event EventBeginPlay
  (Game|Player|SetViewTargetwithBlend (Game|GetPlayerController 0) (Game|GetPlayerCharacter 0) 0.0 "VTBlend_Linear" 0.0 false)
  (bind _outactors (Actor|GetAllActorsOfClass "/Game/workspace/1_mainGame/6_object/BP_Light.BP_Light_C"))
  (Variables|Default|SetLights _outactors)
  (EventDispatchers|BindEventtoOnGetKey (delegate Custom|E_OnGetKey)))

(event EventFIGetKey
  (bind _output_get (Variables|Default|SetKeyNum (+ (Variables|Default|GetKeyNum) 1)))
  (Default|CallOnGetKey _output_get))

(event EventFISetIsSequencePlaying
  (params (isPlaying :type Boolean))
  (Development|PrintString "Hello")
  (Variables|Default|SetisSequencePlaying isPlaying))

(fn ConstructionScript)

(fn FIGetIsSequencePlaying
  (return (Variables|Default|GetisSequencePlaying)))