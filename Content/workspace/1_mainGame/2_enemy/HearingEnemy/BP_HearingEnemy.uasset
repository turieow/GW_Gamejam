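; BP_HearingEnemy is a child enemy Blueprint that tracks heard noises and attacks the player.
; Interface events store noise state and location for querying, and play montages for normal attacks, camera attacks and noticing the player.
; An overridden collision function sphere-checks both hand sockets against Pawns, damages the player on overlap, then clears CollisionEnable.
; The holding interface event also toggles a spotlight's visibility.
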(event EventBeginPlay
  (|CallParentFunction) ; このノードは無効になっているため呼び出せません。\n機能をビルドするにはピンをドラッグしてください。
)

(event Collision|EventActorBeginOverlap
  (params (OtherActor :type Actor%20Object%20Reference))
  (|CallParentFunction OtherActor) ; このノードは無効になっているため呼び出せません。\n機能をビルドするにはピンをドラッグしてください。
)

(event EventFIAttackNormal
  ;[1 1 1] 攻撃通知
  (Animation|Montage|MontagePlay (Components|SkeletalMesh|GetAnimInstance (Variables|Character|GetMesh)) "/Game/workspace/1_mainGame/2_enemy/HearingEnemy/Animation/AM_Anim_Monster_Attack_8.AM_Anim_Monster_Attack_8" 1.0 "MontageLength" 0.0 true))

(event EventFIAttackwithCamera
  ;[1 1 1] 攻撃通知
  (Animation|Montage|MontagePlay (Components|SkeletalMesh|GetAnimInstance (Variables|Character|GetMesh)) "/Game/workspace/1_mainGame/2_enemy/HearingEnemy/Animation/AM_Anim_Monster_Attack_6.AM_Anim_Monster_Attack_6" 1.0 "MontageLength" 0.0 true))

(event EventFISetIsNoise
  (params (location :type Vector :default "0, 0, 0") (getHear :type Boolean))
  ;[1 1 1] 音が聞こえたか
  (Variables|Default|SetisGetNoise getHear)
  (Variables|Default|SetNoiseLocation location))

(event EventFINorticePlayer
  ;[1 1 1] 気づきモーション
  (Animation|Montage|MontagePlay (Components|SkeletalMesh|GetAnimInstance (Variables|Character|GetMesh)) "/Game/workspace/1_mainGame/2_enemy/HearingEnemy/Animation/AM_Anim_Monster_Shout_2.AM_Anim_Monster_Shout_2" 1.0 "MontageLength" 0.0 true))

(event EventFISetIsHolding
  (params (isHolding :type Boolean))
  (bind _holdspotlight (Variables|Default|GetholdSpotLight))
  (|CallParentFunction isHolding)
  (if (Variables|Default|GetisHolding)
    (Rendering|SetVisibility _holdspotlight true false)
    (else
      (Rendering|SetVisibility _holdspotlight false false))))

(fn ConstructionScript
  (|CallParentFunction))

(fn FIGetIsNoise
  (return (Variables|Default|GetisGetNoise) (Variables|Default|GetNoiseLocation)))

(fn FCollisionOverride
  (bind (_outactors _returnvalue) (Collision|SphereOverlapActors (Transformation|GetSocketLocation (Variables|Character|GetMesh) "hand_r") 25.0 (Utilities|Array|MakeArray "ObjectTypeQuery3") 0))
  (if _returnvalue
    (for _array_element _outactors
      (if (== _array_element (Game|Player|GetPlayerPawn 0))
        (Game|Damage|ApplyDamage (Game|Player|GetPlayerPawn 0) (Variables|Default|GetAttackDamage) 0 self :!label _label)
        (Variables|Default|SetCollisionEnable false)
        (|CallParentFunction)
        (else
          (bind (_outactors_2 _returnvalue_2) (Collision|SphereOverlapActors (Transformation|GetSocketLocation (Variables|Character|GetMesh) "hand_l") 25.0 (Utilities|Array|MakeArray "ObjectTypeQuery3") 0))
          (if _returnvalue_2
            (for _array_element_2 _outactors_2
              (if (== _array_element_2 (Game|Player|GetPlayerPawn 0))
                (goto _label)))))))
    (else
      (bind (_outactors_3 _returnvalue_3) (Collision|SphereOverlapActors (Transformation|GetSocketLocation (Variables|Character|GetMesh) "hand_l") 25.0 (Utilities|Array|MakeArray "ObjectTypeQuery3") 0))
      (if _returnvalue_3
        (for _array_element_3 _outactors_3
          (if (== _array_element_3 (Game|Player|GetPlayerPawn 0))
            (Game|Damage|ApplyDamage (Game|Player|GetPlayerPawn 0) (Variables|Default|GetAttackDamage) 0 self)
            (Variables|Default|SetCollisionEnable false)
            (|CallParentFunction)))))))