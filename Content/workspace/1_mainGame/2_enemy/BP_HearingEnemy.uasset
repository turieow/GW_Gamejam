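; BP_HearingEnemy is a hearing enemy Blueprint that holds perception and targeting state for other systems to read.
; Interface events write the player's visibility and whether a noise is heard, along with the noise location.
; Interface getters return those values plus target points and a peep percentage.
; It runs no behavior of its own: Tick is empty and the noise debug print is unconnected.
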(event EventBeginPlay
  (|CallParentFunction) ; このノードは無効になっているため呼び出せません。\n機能をビルドするにはピンをドラッグしてください。
)

(event Collision|EventActorBeginOverlap
  (params (OtherActor :type Actor%20Object%20Reference))
  (|CallParentFunction OtherActor) ; このノードは無効になっているため呼び出せません。\n機能をビルドするにはピンをドラッグしてください。
)

(event EventTick
  (params (DeltaSeconds :type Float%20%28single-precision%29)))

(event EventFISetPlayerVisibility
  (params (visibility :type Boolean))
  (Variables|Default|SetPlayerVisibility visibility))

(event EventFISetIsNoise
  (params (location :type Vector :default "0, 0, 0") (getHear :type Boolean))
  (Variables|Default|SetisGetNoise getHear)
  (Variables|Default|SetNoiseLocation location))

(fn ConstructionScript
  (|CallParentFunction))

(fn FIGetTargetPoints
  (return (Variables|Default|GetTargetPoints)))

(fn FIGetPlayerVisibility
  (return (Variables|Default|GetPlayerVisibility)))

(fn FIGetIsNoise
  (return (Variables|Default|GetisGetNoise) (Variables|Default|GetNoiseLocation)))

(fn FIGetPercentageforPeep
  (return (Variables|Default|GetpercentageForPeep)))