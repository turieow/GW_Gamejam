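; Base enemy character that acts as the interface hub between its AI controller, Behavior Tree and Animation Blueprint.
; It stores visibility, state, holding, patrol target and speed data, forwarding look-at and blend messages to the AnimInstance and animation start/end to the current task.
; While collision is enabled, Tick calls an empty collision override function.
; Noise, lure, peep and voice getters return only defaults, apparently for child enemies to override.
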(event EventBeginPlay
  (Variables|/Script/Engine.CharacterMovementComponent|SetMaxWalkSpeed (Variables|Character|GetCharacterMovement) (Variables|Default|GetWalkSpeed)))

(event EventTick
  (params (DeltaSeconds :type Float%20%28single-precision%29))
  (if (Variables|Default|GetCollisionEnable)
    (CallFunction|FCollisionOverride)))

(event EventFISetPlayerVisibility
  (params (visibility :type Boolean))
  ;[0 0.02954 1] からntroller
  ;;[1 1 1] プレイヤーが見えているか
  (Variables|Default|SetPlayerVisibility visibility))

(event EventFISetEnemyState
  (params (state :type E_EnemyState%20Enum :default "NewEnumerator0"))
  ;[1 0 0.8359] BTから
  ;;[1 1 1] ステートを設定
  (Variables|Default|SetState state))

(event EventFISetAnimationIsBlend
  (params (blend :type Boolean))
  ;[1 0 0.8359] BTから
  ;;[1 1 1] アニメーションをブレンドするか
  (Class|BPIEnemy|FISetAnimationIsBlend(Message) (Components|SkeletalMesh|GetAnimInstance (Variables|Character|GetMesh)) blend))

(event EventFISetLookatAlpha
  (params (alpha :type Float%20%28single-precision%29))
  ;[1 0 0.8359] BTから
  ;;[1 1 1] 首の向き
  (Class|BPIEnemy|FISetLookatAlpha(Message) (Components|SkeletalMesh|GetAnimInstance (Variables|Character|GetMesh)) alpha))

(event EventFISetLookatLocation
  (params (location :type Vector :default "0, 0, 0"))
  ;[1 0 0.8359] BTから
  ;;[1 1 1] 首の向き
  (Class|BPIEnemy|FISetLookatLocation(Message) (Components|SkeletalMesh|GetAnimInstance (Variables|Character|GetMesh)) location))

(event EventFISetMoveSpeed
  (params (speed :type Float%20%28single-precision%29))
  ;[1 0 0.8359] BTから
  ;;[1 1 1] スピードを設定
  (Variables|/Script/Engine.CharacterMovementComponent|SetMaxWalkSpeed (Variables|Character|GetCharacterMovement) speed))

(event EventFISetIsHolding
  (params (isHolding :type Boolean))
  ;[1 0.4255 0] From ABP
  ;;[1 1 1] プレイヤーつかんでいるか
  (Variables|Default|SetisHolding isHolding))

(event EventFIAnimationStart
  ;[1 0.4255 0] From ABP
  ;;[1 1 1] アニメーション開始・終了
  (Class|BPIEnemy|FIAnimationStart(Message) (Variables|Default|GetCurrentTask)))

(event EventFIAnimationEnd
  ;[1 0.4255 0] From ABP
  ;;[1 1 1] アニメーション開始・終了
  (Class|BPIEnemy|FIAnimationEnd(Message) (Variables|Default|GetCurrentTask)))

(event EventFICollisionEnable
  (params (enable :type Boolean))
  ;[1 0.4255 0] From ABP
  ;;[1 1 1] コリジョン発生開始・終了
  (Variables|Default|SetCollisionEnable enable))

(event EventFISetTask
  (params (task :type Object%20Object%20Reference))
  ;[1 0 0.8359] BTから
  ;;[1 1 1] タスクを設定
  (Variables|Default|SetCurrentTask task))

(fn ConstructionScript)

(fn FCollisionOverride)

(fn FIGetAttackDamage
  (return (Variables|Default|GetAttackDamage)))

(fn FIGetCurrentSpeed
  (return (Variables|/Script/Engine.CharacterMovementComponent|GetMaxWalkSpeed (Variables|Character|GetCharacterMovement))))

(fn FIGetEnemySpeed
  (return (Variables|Default|GetWalkSpeed) (Variables|Default|GetRunSpeed)))

(fn FIGetEnemyState
  (return (Variables|Default|GetState)))

(fn FIGetIsHolding
  (return (Variables|Default|GetisHolding)))

(fn FIGetIsNoise
  (return false "0, 0, 0"))

(fn FIGetObikiyoseVoice
  (return 0))

(fn FIGetPercentageforLure
  (return 0.0))

(fn FIGetPercentageforPeep
  (return 0.0))

(fn FIGetPlayerVisibility
  (return (Variables|Default|GetPlayerVisibility)))

(fn FIGetTargetPoints
  (return (Variables|Default|GetTargetPoints)))

(fn FIGetTASUKETEVoice
  (return 0))