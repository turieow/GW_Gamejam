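; BP_FirstEnemy is an enemy Blueprint that holds target points and a player-visibility state, exposed through interface functions.
; An interface event stores the visibility value passed by callers, and two getters return that value and the TargetPoints variable.
; It has no behavior logic of its own: BeginPlay, overlap and Tick are disabled placeholders, and the construction script only calls its parent.
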(event EventBeginPlay
  (|CallParentFunction) ; このノードは無効になっているため呼び出せません。\n機能をビルドするにはピンをドラッグしてください。
)

(event Collision|EventActorBeginOverlap
  (params (OtherActor :type Actor%20Object%20Reference))
  (|CallParentFunction OtherActor) ; このノードは無効になっているため呼び出せません。\n機能をビルドするにはピンをドラッグしてください。
)

(event EventTick
  (params (DeltaSeconds :type Float%20%28single-precision%29))
  (|CallParentFunction DeltaSeconds) ; このノードは無効になっているため呼び出せません。\n機能をビルドするにはピンをドラッグしてください。
)

(event EventFISetPlayerVisibility
  (params (visibility :type Boolean))
  (Variables|Default|SetPlayerVisibility visibility))

(fn ConstructionScript
  (|CallParentFunction))

(fn FIGetTargetPoints
  (return (Variables|Default|GetTargetPoints)))

(fn FIGetPlayerVisibility
  (return (Variables|Default|GetPlayerVisibility)))