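; BP_NormalEnemy is a child enemy Blueprint that supplies the normal monster's animations and melee hit detection.
; Interface events play montages for normal attack, noticing the player, camera attack and tracking-hand animation.
; The FCollisionOverride function sphere-checks the right and left hand sockets for the player pawn.
; A hit applies AttackDamage, clears CollisionEnable and then calls the parent implementation.
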(event EventBeginPlay
  (|CallParentFunction) ; このノードは無効になっているため呼び出せません。\n機能をビルドするにはピンをドラッグしてください。
)

(event Collision|EventActorBeginOverlap
  (params (OtherActor :type Actor%20Object%20Reference)))

(event EventTick
  (params (DeltaSeconds :type Float%20%28single-precision%29)))

(event EventFIAttackNormal
  ;[1 1 1] 攻撃モーション再生
  (Animation|Montage|MontagePlay (Components|SkeletalMesh|GetAnimInstance (Variables|Character|GetMesh)) "/Game/workspace/1_mainGame/2_enemy/NormalEnemy/Animation/AM_Anim_Monster_Attack_9.AM_Anim_Monster_Attack_9" 1.0 "MontageLength" 0.0 true))

(event EventFIAttackwithCamera
  ;[1 1 1] 攻撃モーション再生
  (Animation|Montage|MontagePlay (Components|SkeletalMesh|GetAnimInstance (Variables|Character|GetMesh)) "/Game/workspace/1_mainGame/2_enemy/HearingEnemy/Animation/AM_Anim_Monster_Attack_6.AM_Anim_Monster_Attack_6" 1.0 "MontageLength" 0.0 true))

(event EventFIPlayTrackingHandAnimation
  (Animation|Montage|MontagePlay (Components|SkeletalMesh|GetAnimInstance (Variables|Character|GetMesh)) "/Game/workspace/1_mainGame/2_enemy/HearingEnemy/Animation/AM_Anim_Monster_Attack_2.AM_Anim_Monster_Attack_2" 1.0 "MontageLength" 0.0 true))

(event EventFINorticePlayer
  ;[1 1 1] 気づきモーション
  (Animation|Montage|MontagePlay (Components|SkeletalMesh|GetAnimInstance (Variables|Character|GetMesh)) "/Game/workspace/1_mainGame/2_enemy/NormalEnemy/Animation/AM_Anim_Monster_Shout_2.AM_Anim_Monster_Shout_2" 1.0 "MontageLength" 0.0 true))

(fn ConstructionScript
  (|CallParentFunction))

(fn FCollisionOverride
  (bind (_outactors _returnvalue) (Collision|SphereOverlapActors (Transformation|GetSocketLocation (Variables|Character|GetMesh) "hand_r") 25.0 (Utilities|Array|MakeArray "ObjectTypeQuery3") 0))
  (if _returnvalue
    (for _array_element _outactors
      (if (== _array_element (Game|Player|GetPlayerPawn 0))
        (Game|Damage|ApplyDamage (Game|Player|GetPlayerPawn 0) (Variables|Default|GetAttackDamage) 0 self :!label _label)
        (Variables|Default|SetCollisionEnable false)
        (|CallParentFunction)
        (else
          (bind (_outactors_2 _returnvalue_2) (Collision|SphereOverlapActors (Transformation|GetSocketLocation (Variables|Character|GetMesh) "hand_l") 25.0 (Utilities|Array|MakeArray "ObjectTypeQuery3") 0))
          (if _returnvalue_2
            (for _array_element_2 _outactors_2
              (if (== _array_element_2 (Game|Player|GetPlayerPawn 0))
                (goto _label)))))))
    (else
      (bind (_outactors_3 _returnvalue_3) (Collision|SphereOverlapActors (Transformation|GetSocketLocation (Variables|Character|GetMesh) "hand_l") 25.0 (Utilities|Array|MakeArray "ObjectTypeQuery3") 0))
      (if _returnvalue_3
        (for _array_element_3 _outactors_3
          (if (== _array_element_3 (Game|Player|GetPlayerPawn 0))
            (Game|Damage|ApplyDamage (Game|Player|GetPlayerPawn 0) (Variables|Default|GetAttackDamage) 0 self)
            (Variables|Default|SetCollisionEnable false)
            (|CallParentFunction)))))))